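; Enemy spawner actor that produces waves of enemies at its own transform for as long as it exists.
; On BeginPlay it calls SpawnEnemy, which spawns NumberOfEnemies instances of the configurable Enemy class in a loop.
; The event then waits SpawnDelay and calls itself again, repeating the wave indefinitely with no cap or stop condition.
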(event `self.ReceiveBeginPlay`
  (`self.Spawn Enemy` (`self.Enemy`) (`self.GetTransform`) (`self.Number Of Enemies`)))

(event `Spawn Enemy`
  (params (Enemy :type "Actor Class Reference") (SpawnTransform :type "Transform Structure") (`Number Of Enemies` :type Integer))
  (for _ (range `Number Of Enemies`)
    (`|SpawnActorFromClass` Enemy SpawnTransform "Undefined" "OverrideRootScale" null null))
  (`KismetSystemLibrary.Delay` (`self.Spawn Delay`))
  (`self.Spawn Enemy` (`self.Enemy`) (`self.GetTransform`) (`self.Number Of Enemies`)))

(fn `UserConstructionScript`)